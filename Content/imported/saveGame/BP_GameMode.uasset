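; Game mode blueprint that handles save, load, level-change and restart through a single save slot holding the player character's transform.
; BeginPlay creates the save if missing, otherwise moves the character to the saved transform; the UseSaveLocation check is disconnected.
; SaveGame stores the transform and sets that flag, while ChangeLevels clears it.
; LoadGame restarts the level by console command, and RestartLevel deletes the save first.
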(event `self.ReceiveBeginPlay`
  (bind _returnvalue (`GameplayStatics.DoesSaveGameExist` "save1"))
  (if _returnvalue
    (bind _returnvalue_2 (`GameplayStatics.LoadGameFromSlot` "save1"))
    (bind _asbp_save_game (cast `/Game/imported/saveGame/BP_SaveGame` _returnvalue_2))
    ;[1 1 1] load gamefunctionality
    (bind _asbp_third_person_character (cast `/Game/ThirdPerson/Blueprints/BP_ThirdPersonCharacter` (`GameplayStatics.GetPlayerCharacter` 0)))
    (`SceneComponent.K2_SetWorldTransform` (`Actor.RootComponent` _asbp_third_person_character) (`/Game/imported/saveGame/BP_SaveGame.CharTransform` _asbp_save_game) false false)
    (else
      ;[1 1 1] create save file
      (bind _returnvalue_3 (`GameplayStatics.CreateSaveGameObject` "/Game/imported/saveGame/BP_SaveGame.BP_SaveGame_C"))
      (`GameplayStatics.SaveGameToSlot` _returnvalue_3 "save1"))))

(event `Save Game`
  ;[1 1 1] save game
  (bind _returnvalue (`GameplayStatics.LoadGameFromSlot` "save1"))
  (bind _asbp_save_game (cast `/Game/imported/saveGame/BP_SaveGame` _returnvalue))
  (set `/Game/imported/saveGame/BP_SaveGame.CharTransform` (`self.GetTransform` (cast `/Game/ThirdPerson/Blueprints/BP_ThirdPersonCharacter` (`GameplayStatics.GetPlayerCharacter` 0) :!pure true)) _asbp_save_game)
  (set `/Game/imported/saveGame/BP_SaveGame.UseSaveLocation` true _asbp_save_game)
  (`GameplayStatics.SaveGameToSlot` _asbp_save_game "save1"))

(event `ChangeLevels`
  ;[1 1 1] change levels
  (bind _returnvalue (`GameplayStatics.LoadGameFromSlot` "save1"))
  (bind _asbp_save_game (cast `/Game/imported/saveGame/BP_SaveGame` _returnvalue))
  (set `/Game/imported/saveGame/BP_SaveGame.UseSaveLocation` false _asbp_save_game)
  (`GameplayStatics.SaveGameToSlot` _asbp_save_game "save1"))

(event `Load Game`
  ;[1 1 1] load game
  (`KismetSystemLibrary.ExecuteConsoleCommand` "RestartLevel" null))

(event `RestartLevel`
  ;[1 1 1] delete save and restart
  (`GameplayStatics.DeleteGameInSlot` "save1")
  (`KismetSystemLibrary.ExecuteConsoleCommand` "RestartLevel" null))

(fn `UserConstructionScript`)