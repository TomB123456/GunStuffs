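; Health kit pickup actor that heals the third-person character when the player presses Pick Up nearby.
; Box overlap with BP_ThirdPersonCharacter caches the character and enables input on this actor for player 0, and leaving the box disables it.
; On press, it adds HealingAmount to CurrentHealth, clamped to MaxHealth, then destroys itself.
; At full health it only prints a message and stays in the world.
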(event `self.Box.OnComponentBeginOverlap`
  (params (OverlappedComponent :type "PrimitiveComponent Object Reference") (OtherActor :type "Actor Object Reference") (OtherComp :type "PrimitiveComponent Object Reference") (OtherBodyIndex :type Integer) (bFromSweep :type Boolean) (SweepResult :type "HitResult Structure (by ref)"))
  (bind _asbp_third_person_character (cast `/Game/ThirdPerson/Blueprints/BP_ThirdPersonCharacter` OtherActor))
  (set `self.TPC` _asbp_third_person_character)
  (`self.EnableInput` (`GameplayStatics.GetPlayerController` 0)))

(event `self.Box.OnComponentEndOverlap`
  (params (OverlappedComponent :type "PrimitiveComponent Object Reference") (OtherActor :type "Actor Object Reference") (OtherComp :type "PrimitiveComponent Object Reference") (OtherBodyIndex :type Integer))
  (bind _asbp_third_person_character (cast `/Game/ThirdPerson/Blueprints/BP_ThirdPersonCharacter` OtherActor))
  (set `self.TPC` _asbp_third_person_character)
  (`self.DisableInput` (`GameplayStatics.GetPlayerController` 0)))

(event `InputAction|Pick Up`
  (params (Key :type "Key Structure"))
  (bind _tpc (`self.TPC`))
  (bind _tpc_2 (`self.TPC`))
  (bind _tpc_3 (`self.TPC`))
  (:`Pressed`
    (if (== (`/Game/ThirdPerson/Blueprints/BP_ThirdPersonCharacter.CurrentHealth` _tpc_2) (`/Game/ThirdPerson/Blueprints/BP_ThirdPersonCharacter.MaxHealth` _tpc_2))
      (`KismetSystemLibrary.PrintString` "Health full")
      (elif (> (+ (`/Game/ThirdPerson/Blueprints/BP_ThirdPersonCharacter.CurrentHealth` _tpc_2) (`self.Healing amount`)) (`/Game/ThirdPerson/Blueprints/BP_ThirdPersonCharacter.MaxHealth` _tpc_2))
        (set `/Game/ThirdPerson/Blueprints/BP_ThirdPersonCharacter.CurrentHealth` (`/Game/ThirdPerson/Blueprints/BP_ThirdPersonCharacter.MaxHealth` _tpc) _tpc)
        (`self.K2_DestroyActor`)
        (else
          (set `/Game/ThirdPerson/Blueprints/BP_ThirdPersonCharacter.CurrentHealth` (+ (`/Game/ThirdPerson/Blueprints/BP_ThirdPersonCharacter.CurrentHealth` _tpc_3) (`self.Healing amount`)) _tpc_3)
          (`self.K2_DestroyActor`))))))

(fn `UserConstructionScript`)