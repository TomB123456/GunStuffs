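; Mineable mineral actor that the third-person character breaks apart by holding the Pick Up input while inside its box trigger.
; Overlap toggles input on the actor, and a self-calling Mine event with a short delay lowers MineralHealth by MiningRate while the input is held.
; Health thresholds destroy four rock cube components in turn.
; Once all are gone, the actor destroys itself when the character leaves the box.
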(event `self.Box.OnComponentBeginOverlap`
  (params (OverlappedComponent :type "PrimitiveComponent Object Reference") (OtherActor :type "Actor Object Reference") (OtherComp :type "PrimitiveComponent Object Reference") (OtherBodyIndex :type Integer) (bFromSweep :type Boolean) (SweepResult :type "HitResult Structure (by ref)"))
  (bind _asbp_third_person_character (cast `/Game/ThirdPerson/Blueprints/BP_ThirdPersonCharacter` OtherActor))
  (set `self.TPC` _asbp_third_person_character)
  (`self.EnableInput` (`GameplayStatics.GetPlayerController` 0)))

(event `self.Box.OnComponentEndOverlap`
  (params (OverlappedComponent :type "PrimitiveComponent Object Reference") (OtherActor :type "Actor Object Reference") (OtherComp :type "PrimitiveComponent Object Reference") (OtherBodyIndex :type Integer))
  (bind _asbp_third_person_character (cast `/Game/ThirdPerson/Blueprints/BP_ThirdPersonCharacter` OtherActor))
  (set `self.TPC` _asbp_third_person_character)
  (`self.DisableInput` (`GameplayStatics.GetPlayerController` 0))
  (if (`self.All rocks destroyed?`)
    (`self.K2_DestroyActor`)))

(event `InputAction|Pick Up`
  (params (Key :type "Key Structure"))
  (:`Pressed`
    (set `self.Mining?` true)
    (`self.Mine`))
  (:`Released`
    (set `self.Mining?` false)))

(event `Mine`
  (if (`self.Mining?`)
    (if (<= (`self.Mineral health`) 3.0)
      (`self.Destroy rock1`)
      (if (<= (`self.Mineral health`) 2.0)
        (`self.Destroy rock2`)
        (if (<= (`self.Mineral health`) 1.0)
          (`self.Destroy rock3`)
          (if (<= (`self.Mineral health`) 0.0)
            (`self.Destroy rock4`)
            (set `self.All rocks destroyed?` true)
            (else
              (`KismetSystemLibrary.Delay` 0.5)
              (bind _output_get (set `self.Mineral health` (- (`self.Mineral health`) (`self.Mining rate`))))
              (`KismetSystemLibrary.PrintString` (`KismetStringLibrary.Conv_DoubleToString` _output_get))
              (`self.Mine`)))
          (else
            (`KismetSystemLibrary.Delay` 0.5)
            (bind _output_get_2 (set `self.Mineral health` (- (`self.Mineral health`) (`self.Mining rate`))))
            (`KismetSystemLibrary.PrintString` (`KismetStringLibrary.Conv_DoubleToString` _output_get_2))
            (`self.Mine`)))
        (else
          (`KismetSystemLibrary.Delay` 0.5)
          (set `self.Mineral health` (- (`self.Mineral health`) (`self.Mining rate`)))
          (`self.Mine`)))
      (else
        (`KismetSystemLibrary.Delay` 0.5)
        (bind _output_get_3 (set `self.Mineral health` (- (`self.Mineral health`) (`self.Mining rate`))))
        (`KismetSystemLibrary.PrintString` (`KismetStringLibrary.Conv_DoubleToString` _output_get_3))
        (`self.Mine`)))))

(event `Destroy rock1`
  (if (not (`self.Rock1 destroyed?`))
    (`ActorComponent.K2_DestroyComponent` (`self.Cube`))
    (set `self.Rock1 destroyed?` true)))

(event `Destroy rock2`
  (if (not (`self.Rock2 destroyed?`))
    (`ActorComponent.K2_DestroyComponent` (`self.Cube1`))
    (set `self.Rock2 destroyed?` true)))

(event `Destroy rock3`
  (if (not (`self.Rock3 destroyed?`))
    (`ActorComponent.K2_DestroyComponent` (`self.Cube2`))
    (set `self.Rock3 destroyed?` true)))

(event `Destroy rock4`
  (if (not (`self.Rock4 destroyed?`))
    (`ActorComponent.K2_DestroyComponent` (`self.Cube3`))
    (set `self.Rock4 destroyed?` true)))

(fn `UserConstructionScript`)