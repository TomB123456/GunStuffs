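; Falling stalagmite hazard that drops once when shot by a pistol or rifle projectile.
; A hit moves the Cone to the Cube's position, with CanDamage enabled for the fall, then disables further triggering and destroys the Cube.
; Actor overlaps during that window deal massive damage to the player and zero the health of turrets, drones and melee enemies.
; The pistol branch adds a short delay before damage switches off.
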(event `self.ReceiveActorBeginOverlap`
  (params (OtherActor :type "Actor Object Reference"))
  (bind (_returnvalue_location _returnvalue_rotation) (`KismetMathLibrary.BreakTransform` (`SceneComponent.GetRelativeTransform` (`self.Cone`))))
  (bind _returnvalue_location_2 (`KismetMathLibrary.BreakTransform` (`SceneComponent.GetRelativeTransform` (`self.Cube`))))
  (bind _returnvalue_location_3 (`KismetMathLibrary.BreakTransform` (`SceneComponent.GetRelativeTransform` (`self.Cube`))))
  (bind (_returnvalue_location_4 _returnvalue_rotation_2) (`KismetMathLibrary.BreakTransform` (`SceneComponent.GetRelativeTransform` (`self.Cone`))))
  ;[1 1 1] Pistol
  (if (`KismetMathLibrary.ClassIsChildOf` (`GameplayStatics.GetObjectClass` OtherActor) "/Game/WeaponRelated/FX/PistolProjectile.PistolProjectile_C")
    (if (`self.Can be shot?`)
      (set `self.Can damage?` true)
      (`KismetSystemLibrary.MoveComponentTo` (`self.Cone`) _returnvalue_location_2 _returnvalue_rotation)
      (`KismetSystemLibrary.Delay` 0.1)
      (set `self.Can damage?` false)
      (set `self.Can be shot?` false)
      (`ActorComponent.K2_DestroyComponent` (`self.Cube`)))
    (else
      ;[1 1 1] Rifle
      (if (`KismetMathLibrary.ClassIsChildOf` (`GameplayStatics.GetObjectClass` OtherActor) "/Game/WeaponRelated/FX/RifleProjectile.RifleProjectile_C")
        (if (`self.Can be shot?`)
          (set `self.Can damage?` true)
          (`KismetSystemLibrary.MoveComponentTo` (`self.Cone`) _returnvalue_location_3 _returnvalue_rotation_2)
          (set `self.Can damage?` false)
          (set `self.Can be shot?` false)
          (`ActorComponent.K2_DestroyComponent` (`self.Cube`)))
        (else
          ;[1 1 1] Character
          (if (`KismetMathLibrary.ClassIsChildOf` (`GameplayStatics.GetObjectClass` OtherActor) "/Game/ThirdPerson/Blueprints/BP_ThirdPersonCharacter.BP_ThirdPersonCharacter_C")
            (bind _asbp_third_person_character (cast `/Game/ThirdPerson/Blueprints/BP_ThirdPersonCharacter` OtherActor))
            (if (`self.Can damage?`)
              (set `/Game/ThirdPerson/Blueprints/BP_ThirdPersonCharacter.CurrentHealth` (- (`/Game/ThirdPerson/Blueprints/BP_ThirdPersonCharacter.CurrentHealth` _asbp_third_person_character) 10000.0) _asbp_third_person_character)
              (`/Game/ThirdPerson/Blueprints/BP_ThirdPersonCharacter.Player Damaged` _asbp_third_person_character))
            (else
              ;[1 1 1] Turret
              (if (`KismetMathLibrary.ClassIsChildOf` (`GameplayStatics.GetObjectClass` OtherActor) "/Game/Hostile/Enemy_TurretBP.Enemy_TurretBP_C")
                (bind _asenemy_turret_bp (cast `/Game/Hostile/Enemy_TurretBP` OtherActor))
                (if (`self.Can damage?`)
                  (bind _health (`/Game/Hostile/Enemy_TurretBP.Health` _asenemy_turret_bp))
                  (set `/Game/Hostile/Enemy_TurretBP.Health` (- _health _health) _asenemy_turret_bp))
                (else
                  ;[1 1 1] Drone
                  (if (`KismetMathLibrary.ClassIsChildOf` (`GameplayStatics.GetObjectClass` OtherActor) "/Game/Hostile/Enemy_DroneBP.Enemy_DroneBP_C")
                    (bind _asenemy_drone_bp (cast `/Game/Hostile/Enemy_DroneBP` OtherActor))
                    (if (`self.Can damage?`)
                      (bind _health_2 (`/Game/Hostile/Enemy_DroneBP.Health` _asenemy_drone_bp))
                      (set `/Game/Hostile/Enemy_DroneBP.Health` (- _health_2 _health_2) _asenemy_drone_bp))
                    (else
                      ;[1 1 1] Melee enemy
                      (if (`KismetMathLibrary.ClassIsChildOf` (`GameplayStatics.GetObjectClass` OtherActor) "/Game/Hostile/MeleeEnemy/MeleeEnemy.MeleeEnemy_C")
                        (bind _asmelee_enemy (cast `/Game/Hostile/MeleeEnemy/MeleeEnemy` OtherActor))
                        (if (`self.Can damage?`)
                          (bind _health_3 (`/Game/Hostile/MeleeEnemy/MeleeEnemy.Health` _asmelee_enemy))
                          (set `/Game/Hostile/MeleeEnemy/MeleeEnemy.Health` (- _health_3 _health_3) _asmelee_enemy))))))))))))))

(fn `UserConstructionScript`)