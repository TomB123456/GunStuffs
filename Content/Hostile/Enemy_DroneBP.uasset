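; Enemy drone that patrols between StartHere and EndHere, then shoots at the player once aggroed.
; Chained MoveComponentTo calls drive the patrol; player overlap stops it and starts self-recalling Delay loops that track the player, turn the drone and fire projectiles.
; Overlap and rifle or pistol hits alert its group, while De-agro returns it to its start transform.
; Tick watches Health, then drops rifle ammo, leaves the EnemyGrouper and spawns a dead drone.
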(event `Stop moving`
  (bind _returnvalue_location (`KismetMathLibrary.BreakTransform` (`SceneComponent.GetRelativeTransform` (`self.Start here`))))
  (bind _returnvalue_location_2 (`KismetMathLibrary.BreakTransform` (`SceneComponent.GetRelativeTransform` (`self.End here`))))
  (bind _returnvalue_location_3 (`KismetMathLibrary.BreakTransform` (`SceneComponent.GetRelativeTransform` (`self.Start here`))))
  (`|ExecutionSequence`
    (:`then_0`
      (goto _label :!via `Stop`))
    (:`then_1`
      (goto _label_2 :!via `Stop`))
    (:`then_2`
      (goto _label_3 :!via `Stop`))
    (:`then_3`
      (goto _label_4 :!via `Stop`))))

(event `Begin patrol`
  (bind _returnvalue_location (`KismetMathLibrary.BreakTransform` (`SceneComponent.GetRelativeTransform` (`self.Start here`))))
  (bind _returnvalue_location_2 (`KismetMathLibrary.BreakTransform` (`SceneComponent.GetRelativeTransform` (`self.End here`))))
  (bind _returnvalue_location_3 (`KismetMathLibrary.BreakTransform` (`SceneComponent.GetRelativeTransform` (`self.Start here`))))
  (`KismetSystemLibrary.MoveComponentTo` (`self.Cube`) _returnvalue_location_2 (struct) false false 3.0 :!label _label)
  (`KismetSystemLibrary.Delay` 0.2)
  (if (not (`self.Player detacted?`))
    (`KismetSystemLibrary.Delay` 2.0)
    (`KismetSystemLibrary.MoveComponentTo` (`self.Cube`) _returnvalue_location_2 (struct :`Yaw` 180.0) false false 2.0 :!label _label_2)
    (if (not (`self.Player detacted?`))
      (`KismetSystemLibrary.Delay` 2.0)
      (`KismetSystemLibrary.MoveComponentTo` (`self.Cube`) _returnvalue_location (struct :`Yaw` 180.0) false false 3.0 :!label _label_3)
      (if (not (`self.Player detacted?`))
        (`KismetSystemLibrary.Delay` 2.0)
        (`KismetSystemLibrary.MoveComponentTo` (`self.Cube`) _returnvalue_location_3 (struct) false false 3.0 :!label _label_4)
        (if (not (`self.Player detacted?`))
          (`KismetSystemLibrary.Delay` 2.0)
          (`self.Begin patrol`))))))

(event `self.ReceiveBeginPlay`
  (`|ExecutionSequence`
    (:`then_0`
      (set `self.Start location` (`SceneComponent.GetRelativeTransform` (`self.Cube`))))
    (:`then_1`
      (set `self.Enemy1` self)
      (`self.Begin patrol`))))

(event `SignalGrouper`)

(event `De-agro`
  (bind (_start_location_location _start_location_rotation) (`KismetMathLibrary.BreakTransform` (`self.Start location`)))
  (set `self.Player detacted?` false)
  (`KismetSystemLibrary.MoveComponentTo` (`self.Cube`) _start_location_location _start_location_rotation false false 3.0))

(event `self.ReceiveActorBeginOverlap`
  (params (OtherActor :type "Actor Object Reference"))
  (cast `/Game/ThirdPerson/Blueprints/BP_ThirdPersonCharacter` OtherActor)
  (`self.Agro'd`)
  (`/Game/Hostile/EnemyGrouper.GroupAgro` (`self.Group`)))

(event `Looking at player`
  (if (`self.Player detacted?`)
    (`KismetSystemLibrary.MoveComponentTo` (`self.Cube`) (`self.Actor location when shooting`) (`self.Rotation to look at player`) false false 0.3)
    (`KismetSystemLibrary.Delay` 0.01)
    (`self.Looking at player`)))

(event `Agro'd`
  (bind _returnvalue_location (`KismetMathLibrary.BreakTransform` (`SceneComponent.GetRelativeTransform` (`self.Cube`))))
  (set `self.Player detacted?` true)
  (set `self.Actor location when shooting` _returnvalue_location)
  (`self.Stop moving`)
  (`KismetSystemLibrary.Delay` 0.5)
  (`self.Player range`)
  (`self.Looking at player`)
  (`KismetSystemLibrary.Delay` 1.0)
  (`self.Shooting at player`))

(event `Player range`
  (bind _returnvalue_location (`KismetMathLibrary.BreakTransform` (`SceneComponent.GetRelativeTransform` (`self.Player location cube`))))
  (`KismetSystemLibrary.Delay` 0.01)
  (if (not false)
    (`SceneComponent.K2_SetWorldLocationAndRotation` :`self` (`self.Player location cube`) :`NewLocation` (`self.K2_GetActorLocation` (`GameplayStatics.GetPlayerCharacter` 0)))
    (set `self.Rotation to look at player` (`KismetMathLibrary.FindRelativeLookAtRotation` (`SceneComponent.GetRelativeTransform` (`self.Enemy location cube`)) _returnvalue_location))
    (`self.Player range`)))

(event `Shooting at player`
  (if (`self.Player detacted?`)
    (`|SpawnActorFromClass` "/Game/Hostile/DroneProjectile2.DroneProjectile2_C" (`SceneComponent.K2_GetComponentToWorld` (`self.Aiming`)) "Undefined" "OverrideRootScale" null null)
    (`KismetSystemLibrary.Delay` 3.0)
    (`self.Shooting at player`)))

(event `self.OverlapCollider.OnComponentBeginOverlap`
  (params (OverlappedComponent :type "PrimitiveComponent Object Reference") (OtherActor :type "Actor Object Reference") (OtherComp :type "PrimitiveComponent Object Reference") (OtherBodyIndex :type Integer) (bFromSweep :type Boolean) (SweepResult :type "HitResult Structure (by ref)"))
  (`|ExecutionSequence`
    (:`then_0`
      (bind _asrifle_projectile (cast `/Game/WeaponRelated/FX/RifleProjectile` OtherActor))
      (set `self.Health` (- (`self.Health`) (`/Game/WeaponRelated/FX/RifleProjectile.RifleDamage` _asrifle_projectile)))
      (`/Game/Hostile/EnemyGrouper.GroupAgro` (`self.Group`)))
    (:`then_1`
      (bind _aspistol_projectile (cast `/Game/WeaponRelated/FX/PistolProjectile` OtherActor))
      (set `self.Health` (- (`self.Health`) (`/Game/WeaponRelated/FX/PistolProjectile.PistolDamage` _aspistol_projectile)))
      (`/Game/Hostile/EnemyGrouper.GroupAgro` (`self.Group`)))))

(event `self.ReceiveTick`
  (params (DeltaSeconds :type "Float (single-precision)"))
  (if (<= (`self.Health`) 0.0)
    (`|SpawnActorFromClass` "/Game/WeaponRelated/Ammunition/RifleAmmo.RifleAmmo_C" (`self.GetTransform`) "Undefined" "OverrideRootScale" null null)
    (bind _asenemy_grouper (cast `/Game/Hostile/EnemyGrouper` (`self.Group`)))
    (`KismetArrayLibrary.Array_RemoveItem` (`/Game/Hostile/EnemyGrouper.DroneArray` _asenemy_grouper) self)
    (`|SpawnActorFromClass` "/Game/Hostile/Enemy_Drone_DeadBP.Enemy_Drone_DeadBP_C" (`KismetMathLibrary.MakeTransform` (`SceneComponent.K2_GetComponentLocation` (`self.Cube`)) (`SceneComponent.K2_GetComponentRotation` (`self.Cube`))) "Undefined" "OverrideRootScale" null null)
    (`self.K2_DestroyActor`)))

(fn `UserConstructionScript`)