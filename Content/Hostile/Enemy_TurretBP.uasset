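; Enemy turret that sweeps back and forth until the player overlaps it, then aggros, alerts its group, tracks the player and fires projectiles.
; Searching, targeting and shooting run as self-calling Delay loops gated by PlayerDetected.
; Rifle and pistol hits reduce health and alert the group; Tick handles death, dropping rifle ammo and leaving the EnemyGrouper array.
; The distance-based de-aggro check is disconnected, leaving PlayerDistance empty.
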(event `self.ReceiveBeginPlay`
  (`self.Search mode`))

(event `Search mode`
  ;[1 1 1] Patrol
  (if (not (`self.Player detected?`))
    (`KismetSystemLibrary.MoveComponentTo` (`self.Turret`) (0.0 0.0 0.0) (struct :`Yaw` 180.0) false false 3.5 :!label _label)
    (`KismetSystemLibrary.Delay` 1.0)
    (if (not (`self.Player detected?`))
      (`KismetSystemLibrary.MoveComponentTo` (`self.Turret`) (0.0 0.0 0.0) (struct) false false 3.5 :!label _label_2)
      (`KismetSystemLibrary.Delay` 1.0)
      (if (not (`self.Player detected?`))
        (`self.Search mode`)))))

(event `self.ReceiveActorBeginOverlap`
  (params (OtherActor :type "Actor Object Reference"))
  ;[1 1 1] Player detected
  (cast `/Game/ThirdPerson/Blueprints/BP_ThirdPersonCharacter` OtherActor)
  (`self.Agro'd`)
  (`/Game/Hostile/EnemyGrouper.GroupAgro` (`self.Group`)))

(event `Player detected`
  ;[1 1 1] Patrol
  (`|ExecutionSequence`
    (:`then_0`
      (goto _label :!via `Stop`))
    (:`then_1`
      (goto _label_2 :!via `Stop`))))

(event `Agro'd`
  ;[1 1 1] Player detected
  (set `self.Player detected?` true)
  (`self.Player detected`)
  (`KismetSystemLibrary.Delay` 0.5)
  (`self.Player targeting`)
  (`self.Target player`)
  (`KismetSystemLibrary.Delay` 1.0)
  (`self.Shooting`)
  (`self.Player distance`))

(event `self.OverlapCollider.OnComponentBeginOverlap`
  (params (OverlappedComponent :type "PrimitiveComponent Object Reference") (OtherActor :type "Actor Object Reference") (OtherComp :type "PrimitiveComponent Object Reference") (OtherBodyIndex :type Integer) (bFromSweep :type Boolean) (SweepResult :type "HitResult Structure (by ref)"))
  ;[1 1 1] Taking damage
  (`|ExecutionSequence`
    (:`then_0`
      (bind _asrifle_projectile (cast `/Game/WeaponRelated/FX/RifleProjectile` OtherActor))
      (set `self.Health` (- (`self.Health`) (`/Game/WeaponRelated/FX/RifleProjectile.RifleDamage` _asrifle_projectile)))
      (`/Game/Hostile/EnemyGrouper.GroupAgro` (`self.Group`)))
    (:`then_1`
      (bind _aspistol_projectile (cast `/Game/WeaponRelated/FX/PistolProjectile` OtherActor))
      (set `self.Health` (- (`self.Health`) (`/Game/WeaponRelated/FX/PistolProjectile.PistolDamage` _aspistol_projectile)))
      (`/Game/Hostile/EnemyGrouper.GroupAgro` (`self.Group`)))))

(event `De-agro`
  (set `self.Player detected?` false)
  (`KismetSystemLibrary.Delay` 1.0)
  (`self.Search mode`))

(event `Player targeting`
  (bind _returnvalue_location (`KismetMathLibrary.BreakTransform` (`SceneComponent.GetRelativeTransform` (`self.Turret`))))
  (bind _returnvalue_location_2 (`KismetMathLibrary.BreakTransform` (`SceneComponent.GetRelativeTransform` (`self.player location`))))
  ;[1 1 1] Player targeting
  (if (`self.Player detected?`)
    (`SceneComponent.K2_SetWorldLocation` (`self.player location`) (`self.K2_GetActorLocation` (`GameplayStatics.GetPlayerCharacter` 0)) false false)
    (`KismetSystemLibrary.Delay` 0.01)
    (set `self.Turret location` _returnvalue_location)
    (set `self.Look at player rotation` (`KismetMathLibrary.FindRelativeLookAtRotation` (`SceneComponent.GetRelativeTransform` (`self.Turret location cube`)) _returnvalue_location_2))
    (`self.Player targeting`)))

(event `Player distance`
  ;[1 1 1] Player distance detection
)

(event `self.ReceiveTick`
  (params (DeltaSeconds :type "Float (single-precision)"))
  ;[1 1 1] Death
  (if (<= (`self.Health`) 0.0)
    (`|SpawnActorFromClass` "/Game/WeaponRelated/Ammunition/RifleAmmo.RifleAmmo_C" (`self.GetTransform`) "Undefined" "OverrideRootScale" null null)
    (bind _asenemy_grouper (cast `/Game/Hostile/EnemyGrouper` (`self.Group`)))
    (`KismetArrayLibrary.Array_RemoveItem` (`/Game/Hostile/EnemyGrouper.TurretArray` _asenemy_grouper) self)
    (`self.K2_DestroyActor`)))

(event `Target player`
  ;[1 1 1] Player targeting
  (if (`self.Player detected?`)
    (`KismetSystemLibrary.MoveComponentTo` (`self.Turret`) (`self.Turret location`) (`self.Look at player rotation`) false false 0.5)
    (`KismetSystemLibrary.Delay` 0.01)
    (`self.Target player`)))

(event `Shooting`
  ;[1 1 1] Shooting
  (if (`self.Player detected?`)
    (`|SpawnActorFromClass` "/Game/Hostile/TurretProjectile.TurretProjectile_C" (`SceneComponent.K2_GetComponentToWorld` (`self.Shooting cube`)) "Undefined" "OverrideRootScale" null null)
    (`KismetSystemLibrary.Delay` 1.0)
    (`self.Shooting`)))

(fn `UserConstructionScript`)