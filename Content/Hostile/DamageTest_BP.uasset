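; Test hostile projectile that flies at the player's position captured at spawn and damages the player on contact.
; BeginPlay snaps Targeter to the player, slides Sphere there with MoveComponentTo, then destroys the actor when the move completes.
; Any hit or overlap stops the move.
; If Sphere1 overlaps the third-person character's capsule, it subtracts health, calls PlayerDamaged and destroys itself, with debug prints.
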(event `self.ReceiveBeginPlay`
  (`SceneComponent.K2_SetWorldLocation` (`self.Targeter`) (`self.K2_GetActorLocation` (`GameplayStatics.GetPlayerCharacter` 0)) false false)
  (`KismetSystemLibrary.MoveComponentTo` (`self.Sphere`) (`SceneComponent.RelativeLocation` (`self.Targeter`)) (struct) false false 0.5 :!label _label)
  (`KismetSystemLibrary.Delay` 0.01)
  (`self.K2_DestroyActor`))

(event `self.ReceiveHit`
  (params (MyComp :type "PrimitiveComponent Object Reference") (Other :type "Actor Object Reference") (OtherComp :type "PrimitiveComponent Object Reference") (bSelfMoved :type Boolean) (HitLocation :type "Vector Structure") (HitNormal :type "Vector Structure") (NormalImpulse :type "Vector Structure") (Hit :type "HitResult Structure (by ref)"))
  (goto _label :!via `Stop`))

(event `self.ReceiveActorBeginOverlap`
  (params (OtherActor :type "Actor Object Reference"))
  (`|ExecutionSequence`
    (:`then_0`
      (goto _label :!via `Stop`))
    (:`then_1`
      (bind _asbp_third_person_character (cast `/Game/ThirdPerson/Blueprints/BP_ThirdPersonCharacter` OtherActor)
        (:`then`
          (if (`PrimitiveComponent.IsOverlappingComponent` (`self.Sphere1`) (`Character.CapsuleComponent` _asbp_third_person_character))
            (set `/Game/ThirdPerson/Blueprints/BP_ThirdPersonCharacter.CurrentHealth` (- (`/Game/ThirdPerson/Blueprints/BP_ThirdPersonCharacter.CurrentHealth` _asbp_third_person_character) 10.0) _asbp_third_person_character)
            (`/Game/ThirdPerson/Blueprints/BP_ThirdPersonCharacter.Player Damaged` _asbp_third_person_character)
            (`KismetSystemLibrary.PrintString` "Hit")
            (`self.K2_DestroyActor`)
            (else
              (`KismetSystemLibrary.PrintString` "Test"))))
        (:`CastFailed`
          (`KismetSystemLibrary.PrintString` "Test"))))))

(fn `UserConstructionScript`)